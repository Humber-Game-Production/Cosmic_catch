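; Base ingredient actor for the cooking game that can be chopped into another ingredient.
; Each Chop call advances Progress by scaled delta time and prints it for debugging.
; At full progress it spawns its ChoppedIngredient class in place, hands that to the parent ChoppingDesk as its Item, then destroys itself.
; The Combine event is an empty stub.
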(event `Chop`
  (params (`Delta time` :type "Float (double-precision)"))
  (if (< (`self.Progress`) 1.0)
    (bind _output_get (set `self.Progress` (+ (`self.Progress`) (* `Delta time` 0.5))))
    (`KismetSystemLibrary.PrintString` (`KismetStringLibrary.Conv_DoubleToString` _output_get) true true (struct :`G` 0.66 :`B` 1.0 :`A` 1.0) 0.0)
    (else
      (bind _returnvalue (`|SpawnActorFromClass` (`self.ChoppedIngredient`) (`self.GetTransform`) "Undefined" "OverrideRootScale" null null))
      (bind _aschopping_desk (cast `/Game/Cooking/zaviorsStuff/ChoppingDesk` (`self.GetAttachParentActor`)))
      (set `/Game/Cooking/zaviorsStuff/BP_desk.item` _returnvalue _aschopping_desk)
      (`self.K2_DestroyActor`))))

(event `Combine`
  (params (`second item` :type "Actor Object Reference") (`Player Ref` :type "/Game/Cooking/zaviorsStuff/BP_player Object Reference")))

(fn `UserConstructionScript`)